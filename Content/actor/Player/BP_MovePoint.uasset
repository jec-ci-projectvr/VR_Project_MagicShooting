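; BP_MovePoint is a movement point actor that checks whether a target actor has arrived at it.
; On BeginPlay the target falls back to the player pawn if none is set.
; On overlap it compares the horizontal distance to the target against an arrival threshold and checks that it is the current destination.
; That arrival branch is empty and NextPoint is unused, so nothing happens on arrival.
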(event EventBeginPlay
  (if (not (Utilities|IsValid (Variables|Components|GetTargetActor)))
    (Variables|Components|SetTargetActor (Game|Player|GetPlayerPawn 0))))

(event Collision|EventActorBeginOverlap
  (params (OtherActor :type Actor%20Object%20Reference))
  (bind _reslut (CallFunction|CheckTargetDistance))
  (if (and (< _reslut (Variables|Components|GetArrivalDistance)) (== (Variables|Components|GetTargetDistination) self))
    _))

(event EventTick
  (params (DeltaSeconds :type Float%20%28single-precision%29)))

(fn ConstructionScript)

(fn CheckTargetDistance
  (return (Transformation|GetHorizontalDistanceTo (Variables|Components|GetTargetActor))))