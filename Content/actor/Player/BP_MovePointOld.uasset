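; BP_MovePointOld is a waypoint actor that signals when a target actor, the first player pawn unless another is set, arrives at it.
; Each tick it measures horizontal distance to that target and, if within ArrivalDistance while TargetDistination is this point, calls OnPointArrival with NextPoint.
; The check has no latch, so the call repeats every tick while both conditions hold.
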(event EventBeginPlay
  (if (not (Utilities|IsValid (Variables|Default|GetTargetActor)))
    (Variables|Default|SetTargetActor (Game|Player|GetPlayerPawn 0))))

(event EventTick
  (params (DeltaSeconds :type Float%20%28single-precision%29))
  (bind _reslut (CallFunction|CheckTargetDistance))
  (if (and (< _reslut (Variables|Default|GetArrivalDistance)) (== (Variables|Default|GetTargetDistination) self))
    (Default|CallOnPointArrival (Variables|Default|GetNextPoint))))

(fn ConstructionScript)

(fn CheckTargetDistance
  (return (Transformation|GetHorizontalDistanceTo (Variables|Default|GetTargetActor))))