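; BP_EnemyMonsterNormal is the normal magic monster enemy, an AI-controlled character that fires bullets.
; On spawn it configures EnemyCore and seeds the controller's Blackboard with a brief start flag, attack range and the player as chase target, then takes walk speed from the Blackboard each tick.
; Interface events spawn team-tagged bullets, swap the death material, destroy it, and report deaths to the tutorial widget and GameManager.
; It also destroys itself after falling out of the world.
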(event EventBeginPlay
  (bind _returnvalue (Utilities|Name|MakeLiteralName "isStart"))
  (bind _enemycore (Variables|Default|GetEnemyCore))
  ;[1 1 1] 各値の設定
  (Variables|/Game/actor/Enemy/EnemyCore.EnemyCore_C|SetDieTime _enemycore 2.0)
  (Variables|/Game/actor/Enemy/EnemyCore.EnemyCore_C|SetHitTime _enemycore 0.3)
  (Variables|/Game/actor/Enemy/EnemyCore.EnemyCore_C|SetLife _enemycore 3)
  (bind _asbp_monster_controller (Utilities|Casting|CastToBP_Monster_Controller (Pawn|GetController (Class|AnimInstance|TryGetPawnOwner (Components|SkeletalMesh|GetAnimInstance (Variables|Character|GetMesh))))))
  (bind _output_get (Variables|Default|SetblackBoard (AI|GetBlackboard _asbp_monster_controller)))
  (AI|Components|Blackboard|SetValueasBool _output_get _returnvalue true)
  (AI|Components|Blackboard|SetValueasFloat _output_get (Utilities|Name|MakeLiteralName "AttackRange") (Variables|Default|GetAttackRange))
  (AI|Components|Blackboard|SetValueasObject _output_get (Utilities|Name|MakeLiteralName "ChaseActorKey") (Game|Player|GetPlayerPawn 0))
  (Utilities|FlowControl|Delay 2.0)
  (AI|Components|Blackboard|SetValueasBool _output_get _returnvalue false))

(event Collision|EventActorBeginOverlap
  (params (OtherActor :type Actor%20Object%20Reference)))

(event EventTick
  (params (DeltaSeconds :type Float%20%28single-precision%29))
  (Variables|/Script/Engine.CharacterMovementComponent|SetMaxWalkSpeed (Variables|Character|GetCharacterMovement) (Class|BlackboardComponent|GetValueasFloat (Variables|Default|GetblackBoard) (Utilities|Name|MakeLiteralName "MaxSpeed")))
  ;[1 1 1] 落ちたら消す
  (if (< (.z (Transformation|GetWorldLocation (Variables|Default|GetCapsuleComponent))) -1e+04)
    (Actor|DestroyActor)))

(event EventBPIDieEvent
  (Utilities|FlowControl|Sequence
    (:then_0
      (bind _returnvalue (Actor|GetActorOfClass "/Game/actor/UI/Tutorial_Widget.Tutorial_Widget_C"))
      (if (Utilities|Enum|Equal(Enum) (Variables|/Game/actor/UI/Tutorial_Widget.Tutorial_Widget_C|GettutorialEvent _returnvalue) "NewEnumerator4")
        (Default|CounterPlus _returnvalue)))
    (:then_1
      (bind _outactors (Actor|GetAllActorswithTag "GameManager"))
      (Class|BPIGameManager|BPIEnemyNormalPlus(Message) (Utilities|Array|Get(acopy) _outactors)))))

(event EventBPIEnemyAttack
  (bind _shootingpos (Variables|Default|GetShootingPos))
  (Game|SpawnActorfromClass "/Game/actor/Bullet/EnemyAttack/BP_EnemyBullet.BP_EnemyBullet_C" (Math|Transform|MakeTransform (Transformation|GetWorldLocation _shootingpos) (Transformation|GetWorldRotation _shootingpos)) "Undefined" "MultiplyWithRoot" self (Variables|/Game/actor/Enemy/EnemyCore.EnemyCore_C|GetTeam%20Id (Variables|Default|GetEnemyCore)) 0))

(event EventBPIChangeDieMaterial
  (Rendering|Material|SetMaterial (Variables|Character|GetMesh) 0 "/Game/actor/Enemy/MagicMonster/MI_MonsterNew_Die.MI_MonsterNew_Die"))

(event EventBPIDestroySelf
  (Actor|DestroyActor))

(fn ConstructionScript)

(fn ChangeDieMaterial
  (Rendering|Material|SetMaterial (Variables|Character|GetMesh) 0 "/Game/actor/Enemy/MagicMonster/MI_MonsterNew_Die.MI_MonsterNew_Die"))

(fn BPIHitDieAnim
  (params (anim :type Anim%20Instance%20Object%20Reference))
  (return false false false))

(fn GetTeamId
  (return (Variables|/Game/actor/Enemy/EnemyCore.EnemyCore_C|GetTeam%20Id (Variables|Default|GetEnemyCore))))