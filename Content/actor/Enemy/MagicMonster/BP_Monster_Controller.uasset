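; AI controller for the magic monster enemy, driving it with a behavior tree that targets the player.
; On BeginPlay it loads BB_NPC and, if the player pawn is valid, stores it as the chase target and runs BT_Monster.
; An interface function feeds the animation Blueprint the hit and death states from the pawn's EnemyCore component, plus the blackboard attack flag.
; An interface event stops movement.
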(event EventBeginPlay
  (bind _returnvalue (Game|Player|GetPlayerPawn 0))
  (bind _blackboardcomponent (Class|AIController|UseBlackboard "/Game/actor/Enemy/AI2/BB_NPC.BB_NPC"))
  (Utilities|IsValid _returnvalue
    (:Is%20Valid
      (AI|Components|Blackboard|SetValueasObject _blackboardcomponent (Utilities|Name|MakeLiteralName "ChaseActorKey") _returnvalue)
      (AI|RunBehaviorTree "/Game/actor/Enemy/MagicMonster/BT_Monster.BT_Monster"))))

(event EventTick
  (params (DeltaSeconds :type Float%20%28single-precision%29)))

(event EventBPIStopMovement
  (AI|Navigation|StopMovement self))

(fn ConstructionScript)

(fn BPIHitDieAnim
  (params (anim :type Anim%20Instance%20Object%20Reference))
  (bind _returnvalue (Class|AnimInstance|TryGetPawnOwner anim))
  (bind _returnvalue_2 (Actor|GetComponentbyClass _returnvalue "/Game/actor/Enemy/EnemyCore.EnemyCore_C"))
  (Variables|Default|SetAnimBP_AttackFlag (ScalableFloat|GetValueasBool (AI|GetBlackboard self) (Utilities|Name|MakeLiteralName "AttackFlag")))
  ;[1 1 1] HitとDieの動き
  (if (Utilities|IsValid _returnvalue_2)
    (Variables|Default|SetisHit (Variables|/Game/actor/Enemy/EnemyCore.EnemyCore_C|GetIsHit _returnvalue_2))
    (Variables|Default|SetisDie (Variables|/Game/actor/Enemy/EnemyCore.EnemyCore_C|GetIsDie _returnvalue_2))
    (return (Variables|Default|GetisHit) (Variables|Default|GetisDie) (Variables|Default|GetAnimBP_AttackFlag))))