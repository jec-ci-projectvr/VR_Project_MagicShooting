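; BP_Boss is the boss enemy character, whose DieEvent sends the VR player to the result.
; BeginPlay configures EnemyCore and seeds the AI controller's Blackboard with attack range, chase target and a brief isStart flag.
; Tick takes walk speed from the Blackboard and destroys the boss if it falls too low.
; FireBullet spawns a team-tagged BP_EnemyBullet at ShootingPos; its homing-target logic is left unconnected.
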(event EventBeginPlay
  (bind _returnvalue (Utilities|Name|MakeLiteralName "isStart"))
  (bind _enemycore (Variables|Default|GetEnemyCore))
  ;[1 1 1] 各値の設定
  (bind _returnvalue_2 (Actor|GetActorOfClass "/Game/actor/Player/New/VRCharacter.VRCharacter_C"))
  (Variables|Default|SetPlayer _returnvalue_2)
  (Variables|/Game/actor/Enemy/EnemyCore.EnemyCore_C|SetDieTime _enemycore 2.0)
  (Variables|/Game/actor/Enemy/EnemyCore.EnemyCore_C|SetHitTime _enemycore 0.3)
  (Variables|/Game/actor/Enemy/EnemyCore.EnemyCore_C|SetLife _enemycore 10)
  (bind _asbp_boss_controller (Utilities|Casting|CastToBP_Boss_Controller (Pawn|GetController (Class|AnimInstance|TryGetPawnOwner (Components|SkeletalMesh|GetAnimInstance (Variables|Character|GetMesh))))))
  (bind _output_get (Variables|Default|SetblackBoard (AI|GetBlackboard _asbp_boss_controller)))
  (AI|Components|Blackboard|SetValueasBool _output_get _returnvalue true)
  (AI|Components|Blackboard|SetValueasFloat _output_get (Utilities|Name|MakeLiteralName "AttackRange") (Variables|Default|GetAttackRange))
  (AI|Components|Blackboard|SetValueasObject _output_get (Utilities|Name|MakeLiteralName "ChaseActorKey") (Game|Player|GetPlayerPawn 0))
  (Utilities|FlowControl|Delay 2.0)
  (AI|Components|Blackboard|SetValueasBool _output_get _returnvalue false))

(event Collision|EventActorBeginOverlap
  (params (OtherActor :type Actor%20Object%20Reference)))

(event EventTick
  (params (DeltaSeconds :type Float%20%28single-precision%29))
  (Variables|/Script/Engine.CharacterMovementComponent|SetMaxWalkSpeed (Variables|Character|GetCharacterMovement) (Class|BlackboardComponent|GetValueasFloat (Variables|Default|GetblackBoard) (Utilities|Name|MakeLiteralName "MaxSpeed")))
  ;[1 1 1] 落ちたら消す
  (if (< (.z (Transformation|GetWorldLocation (Variables|Default|GetCapsuleComponent))) -1e+04)
    (Actor|DestroyActor)))

(fn ConstructionScript)

(fn FireBullet
  (bind _shootingpos (Variables|Default|GetShootingPos))
  (bind _returnvalue (Game|SpawnActorfromClass "/Game/actor/Bullet/EnemyAttack/BP_EnemyBullet.BP_EnemyBullet_C" (Math|Transform|MakeTransform (Transformation|GetWorldLocation _shootingpos) (Transformation|GetWorldRotation _shootingpos)) "Undefined" "MultiplyWithRoot" self (Variables|/Game/actor/Enemy/EnemyCore.EnemyCore_C|GetTeam%20Id (Variables|Default|GetEnemyCore)) 0)))

(fn FindHomingTarget
  (bind _outactors (Actor|GetAllActorsOfClasswithTag "/Game/actor/Player/New/VRCharacter.VRCharacter_C" "Player"))
  (for _array_element _outactors
    (return _array_element true))
  (return 0 false))

(fn DieEvent
  (Default|ToResult (Variables|Default|GetPlayer)))

(fn GetTeamId
  (return (Variables|/Game/actor/Enemy/EnemyCore.EnemyCore_C|GetTeam%20Id (Variables|Default|GetEnemyCore))))