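; Base enemy actor Blueprint that tracks life, hit and death states, and exposes a team ID.
; BeHitEvent removes one life, then either flags death with a delayed timer or sets a brief hit flag with a shorter timer.
; Separate events destroy the actor and clear the hit flag.
; Tick calls DestroySelfEvent when the owner, rather than the actor itself, falls below a Z threshold.
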(event Custom|DestroySelf_Event
  (Actor|DestroyActor))

(event Custom|IsHitFalse_Event
  (Variables|Default|SetIsHit false))

(event EventBeginPlay)

(event Collision|EventActorBeginOverlap
  (params (OtherActor :type Actor%20Object%20Reference)))

(event EventTick
  (params (DeltaSeconds :type Float%20%28single-precision%29))
  (if (< (.z (Transformation|GetActorLocation (Components|GetOwner))) -1e+01)
    (CallFunction|DestroySelfEvent)))

(fn ConstructionScript)

(fn BeHitEvent
  (bind _output_get (Variables|Default|SetLife (- (Variables|Default|GetLife) 1.0)))
  (if (<= _output_get 0.0)
    (Variables|Default|SetIsDie true)
    (Utilities|Time|SetTimerbyEvent (EventDispatchers|CreateEvent :!event Custom|DestroySelf_Event) 2.0)
    (else
      (Variables|Default|SetIsHit true)
      (Utilities|Time|SetTimerbyEvent (EventDispatchers|CreateEvent :!event Custom|IsHitFalse_Event) 0.3))))

(fn GetTeamId
  (return (Variables|Default|GetTeam%20Id)))