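; BP_FireWork is a firework actor in the Bullet folder that bursts on a timer.
; On BeginPlay it plays a rocket sound, waits briefly, spawns BP_FireBoom at its location and destroys itself.
; It exposes its TeamId through GetTeamId, but its overlap events are empty.
; Shield and EnemyCore hit logic, including damage and a radial fracture field, is left disconnected and never runs.
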(event OnComponentBeginOverlap(Sphere)
  (params (OverlappedComponent :type Primitive%20Component%20Object%20Reference) (OtherActor :type Actor%20Object%20Reference) (OtherComp :type Primitive%20Component%20Object%20Reference) (OtherBodyIndex :type Integer) (bFromSweep :type Boolean) (SweepResult :type Hit%20Result%20Structure%20%28by%20ref%29)))

(event EventBeginPlay
  ;[1 1 1] サウンドを鳴らす
  (Audio|PlaySoundatLocation "/Game/Sound/SoundEffect/FireWork/rocket-report-and-scream-jr-93060__mp3cut_net_.rocket-report-and-scream-jr-93060__mp3cut_net_" (Transformation|GetActorLocation) "0, 0, 0" 0.7 1.0 0.4 0 0 0 0)
  (Utilities|FlowControl|Delay 2.5)
  (Game|SpawnActorfromClass "/Game/actor/Bullet/FireWork/BP_FireBoom.BP_FireBoom_C" (Math|Conversions|ToTransform(Vector) (Transformation|GetActorLocation)) "Undefined" "MultiplyWithRoot" 0 0)
  (Actor|DestroyActor))

(event Collision|EventActorBeginOverlap
  (params (OtherActor :type Actor%20Object%20Reference)))

(event EventTick
  (params (DeltaSeconds :type Float%20%28single-precision%29)))

(fn ConstructionScript)

(fn GetTeamId
  (return (Variables|Default|GetTeam%20Id)))