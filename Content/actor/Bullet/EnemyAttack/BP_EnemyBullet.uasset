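; BP_EnemyBullet is a team-tagged projectile that plays a fire sound on spawn and explodes on hitting an opposing combatant.
; On overlap it looks for a living EnemyCore component with a different TeamId and calls its hit event.
; The hit also spawns a scaled BP_BoomFire effect and triggers an FS_MasterField radial field at the impact point, then destroys the bullet.
; The graphs contain no movement logic.
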(event EventBeginPlay
  ;[1 1 1] サウンドを鳴らす
  (Audio|PlaySoundatLocation "/Game/Magic_Attacks/Fire/Attack/Fire_AttackF3.Fire_AttackF3" (Transformation|GetActorLocation) "0, 0, 0" 1.0 1.0 0.4 0 0 0 0))

(event Collision|EventActorBeginOverlap
  (params (OtherActor :type Actor%20Object%20Reference))
  (bind _returnvalue (Actor|GetComponentbyClass OtherActor "/Game/actor/Enemy/EnemyCore.EnemyCore_C"))
  (bind _defaultsceneroot (Variables|Default|GetDefaultSceneRoot))
  (bind _returnvalue_2 (Transformation|GetWorldLocation _defaultsceneroot))
  (if (Utilities|IsValid _returnvalue)
    (if (not (Variables|/Game/actor/Enemy/EnemyCore.EnemyCore_C|GetIsDie _returnvalue))
      (if (Utilities|Enum|NotEqual(Enum) (Variables|/Game/actor/Enemy/EnemyCore.EnemyCore_C|GetTeam%20Id _returnvalue) (Variables|Default|GetTeam%20Id))
        (bind _returnvalue_3 (Game|SpawnActorfromClass "/Game/actor/Bullet/Boom/BP_BoomFire.BP_BoomFire_C" (Math|Conversions|ToTransform(Vector) _returnvalue_2) "Undefined" "MultiplyWithRoot" self (Game|Player|GetPlayerPawn 0)))
        (Niagara|SetNiagaraVariable(Float) (Variables|/Game/actor/Bullet/Boom/BP_BoomFire.BP_BoomFire_C|GetBoomVFX _returnvalue_3) "ParticleScale" (Variables|Default|GetParticleSize))
        (Default|BeHitEvent _returnvalue)
        (bind _returnvalue_4 (Game|SpawnActorfromClass "/Engine/EditorResources/FieldNodes/FS_MasterField.FS_MasterField_C" (Math|Transform|MakeTransform _returnvalue_2 "0, 0, 0" "2.000000,2.000000,2.000000") "Undefined" "MultiplyWithRoot" 0 0))
        (Components|Sphere|SetSphereRadius (Variables|/Engine/EditorResources/FieldNodes/FS_MasterField.FS_MasterField_C|GetSphereVolumeCol _returnvalue_4) 5e+01 true)
        (Variables|/Engine/EditorResources/FieldNodes/FS_MasterField.FS_MasterField_C|SetRadial%20Magnitude _returnvalue_4 6e+02)
        (Default|CETrigger _returnvalue_4)
        (Actor|DestroyActor)))))

(event EventTick
  (params (DeltaSeconds :type Float%20%28single-precision%29)))

(fn ConstructionScript)

(fn GetTeamId
  (return (Variables|Default|GetTeam%20Id)))