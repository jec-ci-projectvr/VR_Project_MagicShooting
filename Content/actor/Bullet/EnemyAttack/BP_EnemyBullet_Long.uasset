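; BP_EnemyBullet_Long is an enemy projectile that homes in on the VR player's camera and can be blocked by a shield.
; On BeginPlay it plays a fire sound and sets the tagged player's camera as the ProjectileMovement homing target.
; Sphere overlap with a Shield-tagged component spawns a light explosion, calls the player's BlockEvent and destroys the bullet.
; Team-checked EnemyCore hit and Chaos field logic is disconnected, leaving only shield handling active.
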(event OnComponentBeginOverlap(Sphere)
  (params (OverlappedComponent :type Primitive%20Component%20Object%20Reference) (OtherActor :type Actor%20Object%20Reference) (OtherComp :type Primitive%20Component%20Object%20Reference) (OtherBodyIndex :type Integer) (bFromSweep :type Boolean) (SweepResult :type Hit%20Result%20Structure%20%28by%20ref%29))
  (if (Components|ComponentHasTag OtherComp "Shield")
    (Game|SpawnActorfromClass "/Game/actor/Bullet/Boom/BP_BoomLight.BP_BoomLight_C" (Math|Conversions|ToTransform(Vector) (Transformation|GetWorldLocation (Variables|Default|GetDefaultSceneRoot))) "Undefined" "MultiplyWithRoot" self (Game|Player|GetPlayerPawn 0))
    (Default|BlockEvent (Variables|Default|GetVRCharacter))
    (Actor|DestroyActor)))

(event EventBeginPlay
  ;[1 1 1] サウンドを鳴らす
  (Audio|PlaySoundatLocation "/Game/Magic_Attacks/Fire/Attack/Fire_AttackF3.Fire_AttackF3" (Transformation|GetActorLocation) "0, 0, 0" 1.0 1.0 0.4 0 0 0 0)
  (bind _outactors (Actor|GetAllActorsOfClasswithTag "/Game/actor/Player/New/VRCharacter.VRCharacter_C" "Player"))
  (for _array_element _outactors
    (bind _output_get (Variables|Default|SetVRCharacter _array_element))
    (Variables|/Script/Engine.ProjectileMovementComponent|SetHomingTargetComponent (Variables|Default|GetProjectileMovement) (Variables|/Game/actor/Player/New/VRCharacter.VRCharacter_C|GetCamera _output_get))))

(event Collision|EventActorBeginOverlap
  (params (OtherActor :type Actor%20Object%20Reference)))

(fn ConstructionScript)

(fn GetTeamId
  (return (Variables|Default|GetTeam%20Id)))