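; Base player bullet that plays a random fire sound on spawn and stops homing after one second.
; On overlapping a living EnemyCore of another team, it spawns a scaled explosion, applies Attack damage and destroys itself.
; That hit also spawns a short-lived radial field actor to drive destruction physics.
; Its sphere detects components tagged as enemy shields, spawning a light burst and destroying the bullet.
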(event OnComponentBeginOverlap(Sphere)
  (params (OverlappedComponent :type Primitive%20Component%20Object%20Reference) (OtherActor :type Actor%20Object%20Reference) (OtherComp :type Primitive%20Component%20Object%20Reference) (OtherBodyIndex :type Integer) (bFromSweep :type Boolean) (SweepResult :type Hit%20Result%20Structure%20%28by%20ref%29))
  ;[1 1 1] Bossシールド
  (if (Components|ComponentHasTag OtherComp "Shield")
    (if (Components|ComponentHasTag OtherComp "EnemyComponent")
      (Game|SpawnActorfromClass "/Game/actor/Bullet/Boom/BP_BoomLight.BP_BoomLight_C" (Math|Conversions|ToTransform(Vector) (Transformation|GetWorldLocation (Variables|Default|GetDefaultSceneRoot))) "Undefined" "MultiplyWithRoot" self (Game|Player|GetPlayerPawn 0))
      (Actor|DestroyActor))))

(event EventBeginPlay
  (bind _soundfx (Variables|Default|GetSoundFX))
  ;[1 1 1] サウンドを鳴らす
  (Audio|PlaySoundatLocation (Utilities|Array|Get(acopy) _soundfx (Math|Random|RandomIntegerinRange 0 (- (Utilities|Array|Length _soundfx) 1))) (Transformation|GetActorLocation) "0, 0, 0" 1.5 1.0 0.4 0 0 0 0)
  (Utilities|FlowControl|Delay 1.0)
  (Variables|/Script/Engine.ProjectileMovementComponent|SetbIsHomingProjectile (Variables|Default|GetProjectileMovement) false))

(event Collision|EventActorBeginOverlap
  (params (OtherActor :type Actor%20Object%20Reference))
  (bind _returnvalue (Actor|GetComponentbyClass OtherActor "/Game/actor/Enemy/EnemyCore.EnemyCore_C"))
  (bind _defaultsceneroot (Variables|Default|GetDefaultSceneRoot))
  (bind _returnvalue_2 (Transformation|GetWorldLocation _defaultsceneroot))
  (if (Utilities|IsValid _returnvalue)
    (if (not (Variables|/Game/actor/Enemy/EnemyCore.EnemyCore_C|GetIsDie _returnvalue))
      (if (Utilities|Enum|NotEqual(Enum) (Variables|/Game/actor/Enemy/EnemyCore.EnemyCore_C|GetTeam%20Id _returnvalue) (Variables|Default|GetTeam%20Id))
        (bind _returnvalue_3 (Game|SpawnActorfromClass "/Game/actor/Bullet/Boom/BP_BoomFire.BP_BoomFire_C" (Math|Conversions|ToTransform(Vector) _returnvalue_2) "Undefined" "MultiplyWithRoot" self (Game|Player|GetPlayerPawn 0)))
        (Niagara|SetNiagaraVariable(Float) (Variables|/Game/actor/Bullet/Boom/BP_BoomFire.BP_BoomFire_C|GetBoomVFX _returnvalue_3) "ParticleScale" (Variables|Default|GetParticleSize))
        (Default|BeHitEvent _returnvalue (Variables|Default|GetAttack))
        ;[1 1 1] 粉砕機能の力生成
        (bind _returnvalue_4 (Game|SpawnActorfromClass "/Game/actor/Bullet/FS_Custom_MasterField.FS_Custom_MasterField_C" (Math|Transform|MakeTransform _returnvalue_2 "0, 0, 0" "2.000000,2.000000,2.000000") "Undefined" "MultiplyWithRoot" 0 0))
        (Components|Sphere|SetSphereRadius (Variables|/Game/actor/Bullet/FS_Custom_MasterField.FS_Custom_MasterField_C|GetSphereVolumeCol _returnvalue_4) 5e+01 true)
        (Variables|/Game/actor/Bullet/FS_Custom_MasterField.FS_Custom_MasterField_C|SetRadial%20Magnitude _returnvalue_4 8e+02)
        (Default|CETrigger _returnvalue_4)
        (Default|DestroyTimer _returnvalue_4 0.3)
        (Actor|DestroyActor)))))

(event EventTick
  (params (DeltaSeconds :type Float%20%28single-precision%29)))

(fn ConstructionScript)

(fn GetTeamId
  (return (Variables|Default|GetTeam%20Id)))