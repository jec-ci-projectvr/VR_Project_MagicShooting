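; BP_BoomEnemyDie is a short-lived explosion actor, named for enemy death, that plays a cannon-blast sound and then removes itself.
; On BeginPlay it waits a brief delay, then plays the sound at its location with a Volume variable and a randomized pitch for variety.
; Tick counts a Time variable down by delta seconds and destroys the actor once it drops below zero.
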(event EventBeginPlay
  ;[1 1 1] サウンドを鳴らす
  (Utilities|FlowControl|Delay 0.05)
  (Audio|PlaySoundatLocation "/Game/Sound/SoundEffect/cannon-blast-with-reverb-smartsound-fx-1-00-03__mp3cut_net_.cannon-blast-with-reverb-smartsound-fx-1-00-03__mp3cut_net_" (Transformation|GetActorLocation) "0, 0, 0" (Variables|Default|GetVolume) (Math|Random|RandomFloatinRange 0.9 1.5) 0.0 0 0 0 0))

(event Collision|EventActorBeginOverlap
  (params (OtherActor :type Actor%20Object%20Reference)))

(event EventTick
  (params (DeltaSeconds :type Float%20%28single-precision%29))
  (Variables|Default|SetTime (- (Variables|Default|GetTime) DeltaSeconds))
  (if (< (Variables|Default|GetTime) 0.0)
    (Actor|DestroyActor)))

(fn ConstructionScript)