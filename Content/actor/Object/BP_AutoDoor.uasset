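; BP_AutoDoor is a wooden double gate that swings open automatically when the player walks into its trigger box.
; BeginPlay caches the first actor tagged "Player", and the box's begin-overlap compares the overlapping actor against it.
; A DoOnce then plays the DoorAnim timeline, whose DoorSwing track lerps the right and left leaves' relative yaw in opposite directions.
; No logic closes the gate or resets the DoOnce, so it opens only once.
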(event OnComponentBeginOverlap(Box)
  (params (OverlappedComponent :type Primitive%20Component%20Object%20Reference) (OtherActor :type Actor%20Object%20Reference) (OtherComp :type Primitive%20Component%20Object%20Reference) (OtherBodyIndex :type Integer) (bFromSweep :type Boolean) (SweepResult :type Hit%20Result%20Structure%20%28by%20ref%29))
  (if (== OtherActor (Variables|Default|GetPlayer))
    (Utilities|FlowControl|DoOnce false
      (:Completed
        (bind _doorswing (Timeline|DoorAnim Play)
          (:Update
            (Transformation|SetRelativeRotation (Variables|Default|GetSM_PROP_wall_wood_gate_door_R_01) (Math|Rotator|MakeRotator 0.0 0.0 (Math|Float|Lerp 0.0 -9e+01 _doorswing)) false false)
            (Transformation|SetRelativeRotation (Variables|Default|GetSM_PROP_wall_wood_gate_door_L_01) (Math|Rotator|MakeRotator 0.0 0.0 (Math|Float|Lerp 0.0 9e+01 _doorswing)) false false)))))))

(event EventBeginPlay
  (bind _outactors (Actor|GetAllActorswithTag "Player"))
  (Variables|Default|SetPlayer (Utilities|Array|Get(acopy) _outactors)))

(fn ConstructionScript)